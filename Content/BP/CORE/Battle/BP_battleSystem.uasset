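; Battle system that tracks units on the tile grid and resolves their skill casts.
; It syncs tile occupancy and unit positions on movement and grid changes, destroying units left on unwalkable tiles.
; CastSkill validates range, expands AOE, spawns the animation actor and applies one rolled impact to units hit, triggering debug respawn at zero HP.
; Optional line of sight passes if any of four offset traces to the target is unblocked.
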(event EventBeginPlay
  (bind _grid (Variables|Default|Getgrid))
  (EventDispatchers|BindEventtoOnGridGenerated _grid (EventDispatchers|CreateEvent :!event OnGridGenerated))
  (EventDispatchers|BindEventtoOnTileDataUpdated _grid (EventDispatchers|CreateEvent :!event OnTileDataUpdated)))

(event Collision|EventActorBeginOverlap
  (params (OtherActor :type Actor%20Object%20Reference)))

(event EventTick
  (params (DeltaSeconds :type Float%20%28single-precision%29)))

(fn ConstructionScript)

(fn AddUnittoBattle
  (params (unit :type BP%20Unit%20Object%20Reference) (index :type Int%20Point%20Structure))
  (Utilities|Array|Add (Variables|Default|GetunitInBattle) unit)
  (CallFunction|SetUnitIndexonGrid unit index false)
  (Default|SetGrid unit (Variables|Default|Getgrid))
  (EventDispatchers|BindEventtoOnUnitReachesNewTile unit (EventDispatchers|CreateEvent :!event OnUnitReachedNewTile)))

(fn RemoveUnitfromBattle
  (params (unit :type BP%20Unit%20Object%20Reference) (destroyActor :type Boolean))
  (Utilities|Array|RemoveItem (Variables|Default|GetunitInBattle) unit)
  (CallFunction|SetUnitIndexonGrid unit (Utilities|Struct|MakeIntPoint -999 -999) false)
  (if destroyActor
    (Actor|DestroyActor unit)))

(fn SetUnitIndexonGrid
  (params (unit :type BP%20Unit%20Object%20Reference) (index :type Int%20Point%20Structure) (force :type Boolean))
  (Utilities|FlowControl|Sequence
    (:then_0
      (if (or (!= (Variables|/Game/BP/CORE/Units/BP_unit.BP_unit_C|Getindex unit) index) force)
        (Utilities|FlowControl|Sequence
          (:then_0
            (bind _output_get (LocalVariables|SetpreviousTile (.Value (Utilities|Map|Find (Variables|/Game/BP/CORE/Grid/BP_grid.BP_grid_C|GetgridTiles (Variables|Default|Getgrid)) (Variables|/Game/BP/CORE/Units/BP_unit.BP_unit_C|Getindex unit)))))
            (if (== (.unitOnTile (Utilities|Struct|BreakS_tileData _output_get)) unit)
              (bind _structout (Utilities|Struct|SetmembersinS_tileData (LocalVariables|GetpreviousTile)))
              (Utilities|Map|Add (Variables|/Game/BP/CORE/Grid/BP_grid.BP_grid_C|GetgridTiles (Variables|Default|Getgrid)) (.index (Utilities|Struct|BreakS_tileData _structout)) _structout)))
          (:then_1
            (Variables|/Game/BP/CORE/Units/BP_unit.BP_unit_C|Setindex unit index)
            (if (!= index (Utilities|Struct|MakeIntPoint -999 -999))
              (bind _structout_2 (Utilities|Struct|SetmembersinS_tileData (.Value (Utilities|Map|Find (Variables|/Game/BP/CORE/Grid/BP_grid.BP_grid_C|GetgridTiles (Variables|Default|Getgrid)) index)) unit))
              (Utilities|Map|Add (Variables|/Game/BP/CORE/Grid/BP_grid.BP_grid_C|GetgridTiles (Variables|Default|Getgrid)) (.index (Utilities|Struct|BreakS_tileData _structout_2)) _structout_2)))
          (:then_2
            (Default|CallOnUnitGridIndexChanged unit)))))
    (:then_1
      (Transformation|SetActorLocation unit (select (.ReturnValue (Utilities|Map|Find (Variables|/Game/BP/CORE/Grid/BP_grid.BP_grid_C|GetgridTiles (Variables|Default|Getgrid)) index)) (.location (.transform (Utilities|Struct|BreakS_tileData (.Value (Utilities|Map|Find (Variables|/Game/BP/CORE/Grid/BP_grid.BP_grid_C|GetgridTiles (Variables|Default|Getgrid)) index))))) "-99999.000000,-99999.000000,-99999.000000") false false))))

(fn OnGridGenerated
  (bind _output_get (LocalVariables|SetunitInBattle_temp (Variables|Default|GetunitInBattle)))
  (for _array_element _output_get
    (if (Default|IsTileWalkable (Variables|Default|Getgrid) (Variables|/Game/BP/CORE/Units/BP_unit.BP_unit_C|Getindex _array_element))
      (CallFunction|SetUnitIndexonGrid _array_element (Variables|/Game/BP/CORE/Units/BP_unit.BP_unit_C|Getindex _array_element) true)
      (else
        (CallFunction|RemoveUnitfromBattle _array_element true)))))

(fn OnTileDataUpdated
  (params (index :type Int%20Point%20Structure))
  (bind _output_get (LocalVariables|SetunitInBattle_temp (Variables|Default|GetunitInBattle)))
  (bind _array_element (Utilities|Array|ForEachLoopwithBreak _output_get :!label _label)
    (:LoopBody
      (if (Class|KismetMathLibrary|EqualIntPointIntPoint index (Variables|/Game/BP/CORE/Units/BP_unit.BP_unit_C|Getindex _array_element))
        (if (Default|IsTileWalkable (Variables|Default|Getgrid) (Variables|/Game/BP/CORE/Units/BP_unit.BP_unit_C|Getindex _array_element))
          (CallFunction|SetUnitIndexonGrid _array_element (Variables|/Game/BP/CORE/Units/BP_unit.BP_unit_C|Getindex _array_element) false)
          (goto _label Break)
          (else
            (CallFunction|RemoveUnitfromBattle _array_element true)
            (goto _label Break)))))))

(fn OnUnitReachedNewTile
  (params (unit :type BP%20Unit%20Object%20Reference) (index :type Int%20Point%20Structure))
  (CallFunction|SetUnitIndexonGrid unit index false))

(fn CastSkill
  (params (skill :type E_skill%20Enum :default "NewEnumerator0") (origin%20index :type Int%20Point%20Structure) (target%20index :type Int%20Point%20Structure))
  (bind _grid (Variables|Default|Getgrid))
  (bind _gridtiles (Variables|/Game/BP/CORE/Grid/BP_grid.BP_grid_C|GetgridTiles _grid))
  (bind _value (Utilities|Map|Find _gridtiles origin%20index))
  (bind _unitontile (Utilities|Struct|BreakS_tileData _value))
  (bind _skill_data (CallFunction|GetSkillDatafromSkill skill))
  (LocalVariables|Set_data _skill_data)
  (bind _rangeindexes (CallFunction|GetSkillRange origin%20index (.cast (Utilities|Struct|BreakS_skillData (LocalVariables|Get_data)))))
  (if (Utilities|Array|ContainsItem _rangeindexes target%20index)
    (if (Utilities|Enum|Equal(Enum) (.rangePattern (Utilities|Struct|BreakS_skillData_cast (.castAOE (Utilities|Struct|BreakS_skillData (LocalVariables|Get_data))))) "NewEnumerator0")
      (LocalVariables|Set_attackedIndex (Utilities|Array|MakeArray target%20index))
      (else
        (bind _rangeindexes_2 (CallFunction|GetSkillRange target%20index (.castAOE (Utilities|Struct|BreakS_skillData (LocalVariables|Get_data)))))
        (LocalVariables|Set_attackedIndex _rangeindexes_2)))
    (bind _returnvalue (Game|SpawnActorfromClass (.skillAnimation (Utilities|Struct|BreakS_skillData_assets (.assets (LocalVariables|Get_data)))) (Math|Transform|MakeTransform "0, 0, 0" "0, 0, 0" "1.000000,1.000000,1.000000") "AlwaysSpawn" 0 origin%20index (LocalVariables|Get_attackedIndex) (Variables|Default|Getgrid) target%20index 0))
    (LocalVariables|Set_skillAnimation _returnvalue)
    (Utilities|FlowControl|Sequence
      (:then_0
        (Utilities|IsValid _unitontile
          (:Is%20Valid
            (Default|UnitCastSkill _unitontile target%20index))))
      (:then_1
        (LocalVariables|Set_skillImpactReal (Utilities|Struct|MakeS_skillData_impactReal (CallFunction|MinMaxRandom (Utilities|Struct|BreakS_skillData_impact (.impact (Utilities|Struct|BreakS_skillData (LocalVariables|Get_data)))))))
        (for _array_element (LocalVariables|Get_attackedIndex)
          (bind _output_get (LocalVariables|Set_unit (.unitOnTile (Utilities|Struct|BreakS_tileData (.Value (Utilities|Map|Find (Variables|/Game/BP/CORE/Grid/BP_grid.BP_grid_C|GetgridTiles (Variables|Default|Getgrid)) _array_element))))))
          (Utilities|IsValid _output_get
            (:Is%20Valid
              (if (!= (.HP_current (Utilities|Struct|BreakS_unitData_Stats (.stats (Utilities|Struct|BreakS_unitData (Variables|/Game/BP/CORE/Units/BP_unit.BP_unit_C|GetunitData (LocalVariables|Get_unit)))))) 0)
                (Default|UnitHitbySkill (LocalVariables|Get_unit) (LocalVariables|Get_skillImpactReal) (LocalVariables|Get_skillAnimation))
                (if (== (.HP_current (Utilities|Struct|BreakS_unitData_Stats (.stats (Utilities|Struct|BreakS_unitData (Variables|/Game/BP/CORE/Units/BP_unit.BP_unit_C|GetunitData (LocalVariables|Get_unit)))))) 0)
                  (Default|DebugRespawnAfterDelay (LocalVariables|Get_unit)))))))))))

(fn GetSkillRange
  (params (originIndex :type Int%20Point%20Structure) (cast :type S%20Skill%20Data%20Cast%20Structure))
  (bind (_rangepattern _rangeminmax _lineofsight) (Utilities|Struct|BreakS_skillData_cast cast))
  (bind _indexes (CallFunction|GetIndexesfromPatternandRange originIndex (Variables|/Game/BP/CORE/Grid/BP_grid.BP_grid_C|GetShape (Variables|Default|Getgrid)) _rangepattern _rangeminmax))
  (bind _indexeswithlineofsight (CallFunction|RemoveNotWalkableIndexes :indexes _indexes))
  (if (.requireLineOfSight (Utilities|Struct|BreakS_skillData_LineOfSight _lineofsight))
    (bind _indexeswithlineofsight_2 (CallFunction|RemoveIndexesWithoutLineOfSight originIndex _indexeswithlineofsight cast))
    (return _indexeswithlineofsight_2)
    (else
      (return _indexeswithlineofsight))))

(fn HasLineOfSight
  (params (originIndex :type Int%20Point%20Structure) (targetIndex :type Int%20Point%20Structure) (cast :type S%20Skill%20Data%20Cast%20Structure))
  (bind _grid (Variables|Default|Getgrid))
  (bind _grid_2 (Variables|Default|Getgrid))
  (bind _lineofsight (Utilities|Struct|BreakS_skillData_cast cast))
  (bind _lineofsight_2 (Utilities|Struct|BreakS_skillData_cast cast))
  (bind _gridtiles (Variables|/Game/BP/CORE/Grid/BP_grid.BP_grid_C|GetgridTiles _grid))
  (bind _tile_size (Variables|/Game/BP/CORE/Grid/BP_grid.BP_grid_C|GetTile%20Size _grid_2))
  (bind _heightfromground (Utilities|Struct|BreakS_skillData_LineOfSight _lineofsight))
  (bind _offsetfromcenter (Utilities|Struct|BreakS_skillData_LineOfSight _lineofsight_2))
  (bind _returnvalue (Math|Vector|MakeVector 0.0 0.0 _heightfromground))
  (bind _returnvalue_2 (* _tile_size _offsetfromcenter))
  (LocalVariables|Set_originTile (.Value (Utilities|Map|Find _gridtiles originIndex)))
  (LocalVariables|Set_targetTile (.Value (Utilities|Map|Find _gridtiles targetIndex)))
  (LocalVariables|Set_start (+ (.location (.transform (Utilities|Struct|BreakS_tileData (LocalVariables|Get_originTile)))) _returnvalue))
  (LocalVariables|Set_end (+ _returnvalue (.location (.transform (Utilities|Struct|BreakS_tileData (LocalVariables|Get_targetTile))))))
  (for _array_element (Utilities|Array|MakeArray (Math|Vector2D|MakeVector2D (.x _returnvalue_2) 0.0) (Math|Vector2D|MakeVector2D (- 0.0 (.x _returnvalue_2)) 0.0) (Math|Vector2D|MakeVector2D 0.0 (.y _returnvalue_2)) (Math|Vector2D|MakeVector2D 0.0 (- 0.0 (.y _returnvalue_2))))
    (bind _returnvalue_3 (Collision|LineTraceByChannel (+ (LocalVariables|Get_start) (Math|Conversions|ToVector(Vector2D) _array_element)) (LocalVariables|Get_end) "TraceTypeQuery6" false (Utilities|Array|MakeArray (.unitOnTile (Utilities|Struct|BreakS_tileData (LocalVariables|Get_originTile))) (.unitOnTile (Utilities|Struct|BreakS_tileData (LocalVariables|Get_targetTile)))) (select (.drawDebugLines (Utilities|Struct|BreakS_skillData_LineOfSight (.lineOfSight (Utilities|Struct|BreakS_skillData_cast cast)))) "ForDuration" "None") true "(R=1.000000,G=0.000000,B=0.000000,A=1.000000)" "(R=0.000000,G=1.000000,B=0.000000,A=1.000000)" 2.0))
    (if (not _returnvalue_3)
      (return true)))
  (return false))

(fn RemoveIndexesWithoutLineOfSight
  (params (originIndex :type Int%20Point%20Structure) (indexes :type Array%20of%20Int%20Point%20Structures) (cast :type S%20Skill%20Data%20Cast%20Structure))
  (for _array_element indexes
    (if (CallFunction|HasLineOfSight originIndex _array_element cast)
      (Utilities|Array|Add (LocalVariables|Get_ret) _array_element)))
  (return (LocalVariables|Get_ret)))

(fn RemoveNotWalkableIndexes
  (params (originIndex :type Int%20Point%20Structure) (indexes :type Array%20of%20Int%20Point%20Structures) (cast :type S%20Skill%20Data%20Cast%20Structure))
  (for _array_element indexes
    (if (Default|IsTileWalkable (Variables|Default|Getgrid) _array_element)
      (Utilities|Array|Add (LocalVariables|Get_ret) _array_element)))
  (return (LocalVariables|Get_ret)))