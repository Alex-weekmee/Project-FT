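; BP_skillAnimation is a battle skill effect actor that animates shapes from an origin tile to each attacked grid tile.
; After a short delay, the hidden actor spawns a BP_animatedShape per target, using the grid's shape mesh with randomized red brightness and rate.
; Each finished shape fires a tile-hit dispatcher and removes its index.
; When none remain, it fires a completion dispatcher and destroys itself.
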(event Custom|event_playSkillAnimation
  (bind _grid (Variables|Default|Getgrid))
  (bind _originindex (Variables|Default|GetoriginIndex))
  (bind _returnvalue (Default|GetCurrentShapeData _grid))
  (bind _transform (CallFunction|GetTileTransform _originindex))
  (bind (_meshsize _mesh _meshmaterial) (Utilities|Struct|BreakS_gridShapeData _returnvalue))
  (for _array_element (Variables|Default|GetattackedIndexes)
    (bind _returnvalue_2 (Game|SpawnActorfromClass "/Game/BP/CORE/Battle/skills/skillAnimation/components/BP_animatedShape.BP_animatedShape_C" (Math|Transform|MakeTransform "0, 0, 0" "0, 0, 0" "1.000000,1.000000,1.000000") "AlwaysSpawn" 0 _mesh _meshmaterial (* "(R=1.000000,G=0.000000,B=0.000000,A=1.000000)" (Math|Random|RandomFloatinRange 0.5 1.5)) (Math|Transform|MakeTransform (.location _transform) (.rotation _transform) "0.100000,0.100000,0.100000") (CallFunction|GetTileTransform _array_element) (Math|Random|RandomFloatinRange 0.8 1.2) _array_element 0))
    (EventDispatchers|BindEventtoOnShapeAnimationCompleted _returnvalue_2 (delegate Custom|onShapeAnimationCompleted))))

(event Custom|onShapeAnimationCompleted
  (params (animatedShape :type BP%20Animated%20Shape%20Object%20Reference))
  (bind _index (Variables|/Game/BP/CORE/Battle/skills/skillAnimation/components/BP_animatedShape.BP_animatedShape_C|Getindex animatedShape))
  (bind _attackedindexes (Variables|Default|GetattackedIndexes))
  (Default|CallOnSKillAnimationHitTile self _index)
  (Utilities|Array|RemoveItem _attackedindexes _index)
  (if (== (Utilities|Array|Length _attackedindexes) 0)
    (CallFunction|EventCompleteSkillAnimation)))

(event Custom|Event_CompleteSkillAnimation
  (Rendering|SetActorHiddenInGame true)
  (Default|CallOnSkillAnimationCompleted self)
  (Actor|DestroyActor))

(event EventBeginPlay
  (Rendering|SetActorHiddenInGame true)
  (Utilities|FlowControl|Delay 0.5)
  (CallFunction|EventPlaySkillAnimation))

(fn ConstructionScript)

(fn GetTileTransform
  (params (index :type Int%20Point%20Structure%20%28by%20ref%29))
  (return (.transform (Utilities|Struct|BreakS_tileData (.Value (Utilities|Map|Find (Variables|/Game/BP/CORE/Grid/BP_grid.BP_grid_C|GetgridTiles (Variables|Default|Getgrid)) index))))))