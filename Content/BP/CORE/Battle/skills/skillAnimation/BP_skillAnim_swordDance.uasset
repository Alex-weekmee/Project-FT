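; Skill animation Blueprint that plays the Sword Dance visual at the target tile during battle.
; It moves the actor to that tile and shows a dagger icon in a widget component.
; A single timeline drives the widget's height, draw size, opacity and rotation, then signals skill animation completion when it finishes.
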(event EventBeginPlay
  (|CallParentFunction) ; This node is disabled and will not be called.\nDrag off pins to build functionality.
)

(event Collision|EventActorBeginOverlap
  (params (OtherActor :type Actor%20Object%20Reference)))

(event EventTick
  (params (DeltaSeconds :type Float%20%28single-precision%29)))

(event EventEventPlaySkillAnimation
  (bind _widget_0 (Variables|Default|GetWidget_0))
  (Transformation|SetActorLocation (.location (CallFunction|GetTileTransform (Variables|Default|GettargetIndex))) false false)
  (bind _output_get (Variables|Default|SetwImage (.AsW%20Image (Utilities|Casting|CastToW_image (UserInterface|GetUserWidgetObject (Variables|Default|GetWidget_0))))))
  (Appearance|SetBrushfromTexture (Variables|/Game/BP/CORE/Battle/skills/skillAnimation/components/W_image.W_image_C|GetImage_comp _output_get) "/Game/BP/CORE/Battle/skills/skillAnimation/assets/ICON_dagger.ICON_dagger" false)
  (bind (_direction _locationz _drawsize _opacity _rotation) (Timeline|Timeline_runChickenRun PlayFromStart)
    (:Update
      (Transformation|SetRelativeTransform _widget_0 (Math|Transform|MakeTransform (Math|Vector|MakeVector -1e+02 0.0 _locationz) "0, 0, 0" "1.000000,1.000000,1.000000") false false)
      (Class|WidgetComponent|SetDrawSize _widget_0 (Math|Vector2D|MakeVector2D _drawsize _drawsize))
      (Widget|SetRenderOpacity (Variables|Default|GetwImage) _opacity)
      (Class|Widget|SetRenderTransformAngle (Variables|Default|GetwImage) _rotation))
    (:Finished
      (CallFunction|EventCompleteSkillAnimation))))

(fn ConstructionScript
  (|CallParentFunction))