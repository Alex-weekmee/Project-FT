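; Skill animation actor for a wind gust attack in tile-based battle, with three static meshes tinted in blue-violet shades.
; After a short delay it signals a hit on the target tile, then spawns a growing BP_animatedWindGust from there toward each other attacked tile.
; Each gust's completion callback signals a hit and removes its index from AttackedIndexes, completing the skill animation when the list empties.
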(event Custom|OnWindAnimationCompleted
  (params (animatedShape :type BP%20Animated%20Wind%20Gust%20Object%20Reference))
  (bind _attackedindexes (Variables|Default|GetattackedIndexes))
  (Default|CallOnSKillAnimationHitTile self)
  (Utilities|Array|RemoveItem _attackedindexes (Variables|/Game/BP/CORE/Battle/skills/skillAnimation/components/BP_animatedWindGust.BP_animatedWindGust_C|Getindex animatedShape))
  (if (== (Utilities|Array|Length _attackedindexes) 0)
    (CallFunction|EventCompleteSkillAnimation)))

(event EventBeginPlay
  (|CallParentFunction) ; This node is disabled and will not be called.\nDrag off pins to build functionality.
)

(event Collision|EventActorBeginOverlap
  (params (OtherActor :type Actor%20Object%20Reference)))

(event EventTick
  (params (DeltaSeconds :type Float%20%28single-precision%29)))

(event EventEventPlaySkillAnimation
  (bind _targetindex (Variables|Default|GettargetIndex))
  (bind _transform (CallFunction|GetTileTransform _targetindex))
  (Utilities|FlowControl|Delay 0.2)
  (Default|CallOnSKillAnimationHitTile self (Variables|Default|GettargetIndex))
  (Utilities|Array|RemoveItem (Variables|Default|GetattackedIndexes) (Variables|Default|GettargetIndex))
  (for _array_element (Variables|Default|GetattackedIndexes)
    (bind _returnvalue (Game|SpawnActorfromClass "/Game/BP/CORE/Battle/skills/skillAnimation/components/BP_animatedWindGust.BP_animatedWindGust_C" (Math|Transform|MakeTransform "0, 0, 0" "0, 0, 0" "1.000000,1.000000,1.000000") "Undefined" 0 (Math|Transform|MakeTransform (.location _transform) (Math|Rotator|FindLookatRotation (.location _transform) (.location (CallFunction|GetTileTransform _array_element))) "0.500000,0.500000,0.500000") (Math|Transform|MakeTransform (.location (CallFunction|GetTileTransform _array_element)) (Math|Rotator|FindLookatRotation (.location _transform) (.location (CallFunction|GetTileTransform _array_element))) "1.200000,1.200000,1.200000") 1.0 _array_element 0))
    (EventDispatchers|BindEventtoOnShapeAnimationCompleted _returnvalue (delegate Custom|OnWindAnimationCompleted))))

(fn ConstructionScript
  (|CallParentFunction)
  (Rendering|Material|SetVectorParameterValueonMaterials (Variables|Default|GetStaticMesh) "Color" (Math|Conversions|ToVector(LinearColor) "(R=0.221615,G=0.072917,B=1.000000,A=1.000000)"))
  (Rendering|Material|SetVectorParameterValueonMaterials (Variables|Default|GetStaticMesh1) "Color" (Math|Conversions|ToVector(LinearColor) "(R=0.387787,G=0.270833,B=1.000000,A=1.000000)"))
  (Rendering|Material|SetVectorParameterValueonMaterials (Variables|Default|GetStaticMesh2) "Color" (Math|Conversions|ToVector(LinearColor) "(R=0.160393,G=0.000000,B=1.000000,A=1.000000)")))