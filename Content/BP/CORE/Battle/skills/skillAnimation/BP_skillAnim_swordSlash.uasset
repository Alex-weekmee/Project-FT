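; Sword slash skill animation actor for tile-based battles.
; When played, it moves to the origin tile and faces the target tile, deriving the rotation from the two tile indices rather than world positions.
; A timeline then drives the pitch and uniform scale of the AnimRorationScale component to animate the slash, and signals skill animation completion when it finishes.
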(event EventBeginPlay
  (|CallParentFunction) ; This node is disabled and will not be called.\nDrag off pins to build functionality.
)

(event Collision|EventActorBeginOverlap
  (params (OtherActor :type Actor%20Object%20Reference))
  (|CallParentFunction OtherActor) ; This node is disabled and will not be called.\nDrag off pins to build functionality.
)

(event EventTick
  (params (DeltaSeconds :type Float%20%28single-precision%29))
  (|CallParentFunction DeltaSeconds) ; This node is disabled and will not be called.\nDrag off pins to build functionality.
)

(event EventEventPlaySkillAnimation
  (bind _anim_rorationscale (Variables|Default|Getanim_rorationScale))
  (Transformation|SetActorLocationAndRotation (.location (CallFunction|GetTileTransform (Variables|Default|GetoriginIndex))) (Math|Rotator|FindLookatRotation (Math|Conversions|ToVector(Vector2D) (Math|Conversions|ToVector2D(IntPoint) (Variables|Default|GetoriginIndex))) (Math|Conversions|ToVector(Vector2D) (Math|Conversions|ToVector2D(IntPoint) (Variables|Default|GettargetIndex)))))
  (bind (_direction _rotationy _scale) (Timeline|Timeline_swordSlash PlayFromStart)
    (:Update
      (Transformation|SetRelativeRotation _anim_rorationscale (Math|Rotator|MakeRotator 0.0 _rotationy 0.0) false false)
      (Transformation|SetRelativeScale3D _anim_rorationscale (Math|Conversions|ToVector(Float) _scale)))
    (:Finished
      (CallFunction|EventCompleteSkillAnimation))))

(fn ConstructionScript
  (|CallParentFunction))