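; Skill animation actor that flies a short-range arrow from an origin tile to a target tile in battle.
; On play, it aims at the target, waits briefly, then unhides and starts a timeline.
; The timeline lerps location between tiles with a height offset and drives pitch and scale on a child component.
; It signals the tile hit once, late in playback, and completes the skill animation when finished.
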(event EventBeginPlay
  (|CallParentFunction) ; This node is disabled and will not be called.\nDrag off pins to build functionality.
)

(event Collision|EventActorBeginOverlap
  (params (OtherActor :type Actor%20Object%20Reference)))

(event EventTick
  (params (DeltaSeconds :type Float%20%28single-precision%29)))

(event EventEventPlaySkillAnimation
  (bind _anim_rorationscale (Variables|Default|Getanim_rorationScale))
  (Transformation|SetActorLocationAndRotation (.location (CallFunction|GetTileTransform (Variables|Default|GetoriginIndex))) (Math|Rotator|FindLookatRotation (Math|Conversions|ToVector(Vector2D) (Math|Conversions|ToVector2D(IntPoint) (Variables|Default|GetoriginIndex))) (Math|Conversions|ToVector(Vector2D) (Math|Conversions|ToVector2D(IntPoint) (Variables|Default|GettargetIndex)))))
  (Utilities|FlowControl|Delay 1.45)
  (Rendering|SetActorHiddenInGame false)
  (bind (_direction _actorlocation _locationz _rotationy _scale) (Timeline|Timeline_shortRangedArrow PlayFromStart)
    (:Update
      (Transformation|SetActorLocation (+ (Math|Vector|Lerp(Vector) (.location (CallFunction|GetTileTransform (Variables|Default|GetoriginIndex))) (.location (CallFunction|GetTileTransform (Variables|Default|GettargetIndex))) _actorlocation) (Math|Vector|MakeVector 0.0 0.0 _locationz)) false false)
      (Transformation|SetRelativeRotation _anim_rorationscale (Math|Rotator|MakeRotator 0.0 _rotationy 0.0) false false)
      (Transformation|SetRelativeScale3D _anim_rorationscale (Math|Conversions|ToVector(Float) _scale))
      (if (>= (Components|Timeline|GetPlaybackPosition (Variables|Default|GetTimeline_shortRangedArrow)) 0.75)
        (Utilities|FlowControl|DoOnce false
          (:Completed
            (Default|CallOnSKillAnimationHitTile self (Variables|Default|GettargetIndex))))))
    (:Finished
      (CallFunction|EventCompleteSkillAnimation))))

(fn ConstructionScript
  (|CallParentFunction))