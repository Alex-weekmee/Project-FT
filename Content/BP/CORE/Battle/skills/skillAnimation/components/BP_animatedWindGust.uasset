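; Animated wind gust effect actor for battle skill animations, which plays once and removes itself.
; Construction creates two translucent dynamic materials tinted orange-red with randomized brightness.
; On BeginPlay a rate-adjusted timeline lerps the actor from origin to target transform while driving material opacity.
; When the timeline finishes, it fires the shape-animation-completed event, then destroys itself after a short delay.
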(event EventBeginPlay
  (Components|Timeline|SetPlayRate (Variables|Default|GetTimeline) (Variables|Default|GetNew%20Rate))
  (bind (_direction _tranformalpha _opacity) (Timeline|Timeline PlayFromStart)
    (:Update
      (Transformation|SetActorTransform (Math|Transform|Lerp(Transform) (Variables|Default|GetoriginTransform) (Variables|Default|GettargetTransform) _tranformalpha))
      (Rendering|Material|SetScalarParameterValueonMaterials (Variables|Default|GetanimatedWindGust) "Opacity" _opacity))
    (:Finished
      (Default|CallOnShapeAnimationCompleted self)
      (Utilities|FlowControl|Delay 0.5)
      (Actor|DestroyActor))))

(fn ConstructionScript
  (bind _returnvalue (Rendering|Material|CreateDynamicMaterialInstance (Variables|Default|GetanimatedWindGust) 0 "/Game/Art/Materials/M_TranslucentColor.M_TranslucentColor" "None" :!class /Script/Engine.PrimitiveComponent))
  (Rendering|Material|SetVectorParameterValue _returnvalue "Color" (* "(R=1.000000,G=0.142179,B=0.000000,A=1.000000)" (Math|Random|RandomFloatinRange 0.8 1.5)) :!class /Script/Engine.MaterialInstanceDynamic)
  (bind _returnvalue_2 (Rendering|Material|CreateDynamicMaterialInstance (Variables|Default|GetanimatedWindGust) 1 "/Game/Art/Materials/M_TranslucentColor.M_TranslucentColor" "None" :!class /Script/Engine.PrimitiveComponent))
  (Rendering|Material|SetVectorParameterValue _returnvalue_2 "Color" (* "(R=1.000000,G=0.053420,B=0.000000,A=1.000000)" (Math|Random|RandomFloatinRange 0.8 1.5)) :!class /Script/Engine.MaterialInstanceDynamic))