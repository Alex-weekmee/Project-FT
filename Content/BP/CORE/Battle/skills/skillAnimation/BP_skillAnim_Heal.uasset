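; Skill animation Blueprint for the Heal battle skill, showing a green mesh effect on the target tile.
; The construction script tints the meshes in different shades of green through material parameters.
; On play, it moves to the target tile and runs a timeline (named darkWave) that drives rotation, scale and mesh opacity.
; When the timeline finishes, it calls the skill animation completion event; no healing logic lives here.
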(event EventBeginPlay
  (|CallParentFunction) ; This node is disabled and will not be called.\nDrag off pins to build functionality.
)

(event Collision|EventActorBeginOverlap
  (params (OtherActor :type Actor%20Object%20Reference)))

(event EventTick
  (params (DeltaSeconds :type Float%20%28single-precision%29)))

(event EventEventPlaySkillAnimation
  (bind _anim_rotationscale (Variables|Default|Getanim_rotationScale))
  (Transformation|SetActorLocation (.location (CallFunction|GetTileTransform (Variables|Default|GettargetIndex))) false false)
  (bind (_direction _opacity _scale _rotation) (Timeline|Timeline_darkWave PlayFromStart)
    (:Update
      (Transformation|SetRelativeRotation _anim_rotationscale (Math|Rotator|MakeRotator 0.0 0.0 _rotation) false false)
      (Transformation|SetRelativeScale3D _anim_rotationscale _scale)
      (Rendering|Material|SetScalarParameterValueonMaterials (Variables|Default|GetStaticMesh) "Opacity" _opacity))
    (:Finished
      (CallFunction|EventCompleteSkillAnimation))))

(fn ConstructionScript
  (|CallParentFunction)
  (Rendering|Material|SetVectorParameterValueonMaterials (Variables|Default|GetStaticMesh) "Color" (Math|Conversions|ToVector(LinearColor) "(R=0.072917,G=1.000000,B=0.196528,A=1.000000)"))
  (Rendering|Material|SetVectorParameterValueonMaterials (Variables|Default|GetStaticMesh1) "Color" (Math|Conversions|ToVector(LinearColor) "(R=0.270833,G=1.000000,B=0.368055,A=1.000000)"))
  (Rendering|Material|SetVectorParameterValueonMaterials (Variables|Default|GetStaticMesh2) "Color" (Math|Conversions|ToVector(LinearColor) "(R=0.000000,G=1.000000,B=0.133333,A=1.000000)")))