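; Skill animation actor for the battle "dark wave" skill, playing a scaling, fading purple-blue wave effect on the target tile.
; When played, it moves to the target tile and runs a timeline that drives the AnimScale component's scale and the opacity of three meshes' materials.
; The construction script tints each mesh a different blue-violet shade, and the timeline's end signals skill animation completion.
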(event EventBeginPlay
  (|CallParentFunction) ; This node is disabled and will not be called.\nDrag off pins to build functionality.
)

(event Collision|EventActorBeginOverlap
  (params (OtherActor :type Actor%20Object%20Reference)))

(event EventTick
  (params (DeltaSeconds :type Float%20%28single-precision%29)))

(event EventEventPlaySkillAnimation
  (Transformation|SetActorLocation (.location (CallFunction|GetTileTransform (Variables|Default|GettargetIndex))) false false)
  (bind (_direction _opacity _scale) (Timeline|Timeline_darkWave PlayFromStart)
    (:Update
      (Transformation|SetRelativeScale3D (Variables|Default|Getanim_scale) _scale)
      (Rendering|Material|SetScalarParameterValueonMaterials (Variables|Default|GetStaticMesh) "Opacity" _opacity))
    (:Finished
      (CallFunction|EventCompleteSkillAnimation))))

(fn ConstructionScript
  (|CallParentFunction)
  (Rendering|Material|SetVectorParameterValueonMaterials (Variables|Default|GetStaticMesh) "Color" (Math|Conversions|ToVector(LinearColor) "(R=0.221615,G=0.072917,B=1.000000,A=1.000000)"))
  (Rendering|Material|SetVectorParameterValueonMaterials (Variables|Default|GetStaticMesh1) "Color" (Math|Conversions|ToVector(LinearColor) "(R=0.387787,G=0.270833,B=1.000000,A=1.000000)"))
  (Rendering|Material|SetVectorParameterValueonMaterials (Variables|Default|GetStaticMesh2) "Color" (Math|Conversions|ToVector(LinearColor) "(R=0.160393,G=0.000000,B=1.000000,A=1.000000)")))