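; Battle skill animation actor for a knife throw that flies from the origin tile to the target tile.
; When played, it snaps to the origin tile, facing along the grid direction between the two indices.
; A timeline lerps the actor between the tiles while driving a child component's height, pitch and uniform scale.
; When the timeline finishes, it signals that the skill animation is complete.
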(event EventBeginPlay
  (|CallParentFunction) ; This node is disabled and will not be called.\nDrag off pins to build functionality.
)

(event Collision|EventActorBeginOverlap
  (params (OtherActor :type Actor%20Object%20Reference)))

(event EventTick
  (params (DeltaSeconds :type Float%20%28single-precision%29)))

(event EventEventPlaySkillAnimation
  (Transformation|SetActorLocationAndRotation (.location (CallFunction|GetTileTransform (Variables|Default|GetoriginIndex))) (Math|Rotator|FindLookatRotation (Math|Conversions|ToVector(Vector2D) (Math|Conversions|ToVector2D(IntPoint) (Variables|Default|GetoriginIndex))) (Math|Conversions|ToVector(Vector2D) (Math|Conversions|ToVector2D(IntPoint) (Variables|Default|GettargetIndex)))))
  (bind (_direction _actorlocation _locationz _rotationy _scale) (Timeline|Timeline_knifeThrow PlayFromStart)
    (:Update
      (Transformation|SetActorLocation (Math|Vector|Lerp(Vector) (.location (CallFunction|GetTileTransform (Variables|Default|GetoriginIndex))) (.location (CallFunction|GetTileTransform (Variables|Default|GettargetIndex))) _actorlocation) false false)
      (Transformation|SetRelativeTransform (Variables|Default|Getanim_rorationScale) (Math|Transform|MakeTransform (Math|Vector|MakeVector 0.0 0.0 _locationz) (Math|Rotator|MakeRotator 0.0 _rotationy 0.0) (Math|Conversions|ToVector(Float) _scale)) false false))
    (:Finished
      (CallFunction|EventCompleteSkillAnimation))))

(fn ConstructionScript
  (|CallParentFunction))