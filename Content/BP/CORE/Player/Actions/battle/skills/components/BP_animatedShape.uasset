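; BP_animatedShape is a short-lived battle-skill visual actor that animates a configurable mesh from an origin transform to a target transform.
; On BeginPlay it applies the mesh, material and color, then plays a timeline at a configurable rate.
; The timeline interpolates location, rotation and scale, adding a fixed vertical lift plus a curve-driven height offset.
; When finished, it broadcasts ShapeAnimationCompleted and destroys itself after a short delay.
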(event EventBeginPlay
  (bind _animatedshape (Variables|Default|GetanimatedShape))
  (Components|StaticMesh|SetStaticMesh _animatedshape (Variables|Default|Getmesh))
  (Rendering|Material|SetMaterial _animatedshape 0 (Variables|Default|Getmaterial))
  (Rendering|Material|SetVectorParameterValueonMaterials (Variables|Default|GetanimatedShape) "Color" (Math|Conversions|ToVector(LinearColor) (Variables|Default|Getcolor)))
  (Components|Timeline|SetPlayRate (Variables|Default|GetTimeline) (Variables|Default|GetNew%20Rate))
  (bind (_direction _tranformalpha _heightoffset) (Timeline|Timeline PlayFromStart)
    (:Update
      (Transformation|SetActorTransform (Math|Transform|MakeTransform (+ (.location (Math|Transform|Lerp(Transform) (Variables|Default|GetoriginTransform) (Variables|Default|GettargetTransform) _tranformalpha)) "0.000000,0.000000,100.000000" (Math|Vector|MakeVector 0.0 0.0 _heightoffset)) (.rotation (Math|Transform|Lerp(Transform) (Variables|Default|GetoriginTransform) (Variables|Default|GettargetTransform) _tranformalpha)) (.scale (Math|Transform|Lerp(Transform) (Variables|Default|GetoriginTransform) (Variables|Default|GettargetTransform) _tranformalpha)))))
    (:Finished
      (Default|CallOnShapeAnimationCompleted self)
      (Utilities|FlowControl|Delay 0.5)
      (Actor|DestroyActor))))

(fn ConstructionScript)