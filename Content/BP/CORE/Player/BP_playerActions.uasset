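; Player input actor that tracks the grid tile under the cursor and runs the selected left- and right-click actions on it.
; Tick updates the hovered tile, moves its hover state on the grid, and re-runs held-button actions whenever the tile changes, allowing drag application.
; Actions are swappable spawned actors: SetSelectedActions destroys the old ones, spawns the new classes with a back-reference, and broadcasts the change.
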(event Custom|OnHoveredTileChanged
  (Utilities|FlowControl|Sequence
    (:then_0
      (if (Variables|Default|GetisLeftClickDown)
        (Utilities|IsValid (Variables|Default|GetselectedAction_leftClick)
          (:Is%20Valid
            (Default|ExecuteAction (Variables|Default|GetselectedAction_leftClick) (Variables|Default|GethoveredTile))))))
    (:then_1
      (if (Variables|Default|GetisRightClickDown)
        (Utilities|IsValid (Variables|Default|GetselectedAction_rightClick)
          (:Is%20Valid
            (Default|ExecuteAction (Variables|Default|GetselectedAction_rightClick) (Variables|Default|GethoveredTile))))))))

(event EventBeginPlay
  (bind _returnvalue (Actor|GetActorOfClass "/Game/BP/CORE/Grid/BP_grid.BP_grid_C"))
  (Variables|Default|Setgrid _returnvalue)
  (bind _returnvalue_2 (Actor|GetActorOfClass "/Game/BP/CORE/Battle/BP_battleSystem.BP_battleSystem_C"))
  (Variables|Default|SetcombatSystem _returnvalue_2)
  (Input|EnableInput (Game|GetPlayerController 0)))

(event EventTick
  (params (DeltaSeconds :type Float%20%28single-precision%29))
  (CallFunction|UpdateHoveredTile))

(event Input|MouseEvents|LeftMouseButton
  (params (Key :type Key%20Structure :default "None"))
  (:Pressed
    (CallFunction|UpdateHoveredTile)
    (Variables|Default|SetisLeftClickDown true)
    (Utilities|IsValid (Variables|Default|GetselectedAction_leftClick)
      (:Is%20Valid
        (Default|ExecuteAction (Variables|Default|GetselectedAction_leftClick) (Variables|Default|GethoveredTile)))))
  (:Released
    (Variables|Default|SetisLeftClickDown false)))

(event Input|MouseEvents|RightMouseButton
  (params (Key :type Key%20Structure :default "None"))
  (:Pressed
    (CallFunction|UpdateHoveredTile)
    (Variables|Default|SetisRightClickDown true)
    (Utilities|IsValid (Variables|Default|GetselectedAction_rightClick)
      (:Is%20Valid
        (Default|ExecuteAction (Variables|Default|GetselectedAction_rightClick) (Variables|Default|GethoveredTile)))))
  (:Released
    (Variables|Default|SetisRightClickDown false)))

(fn ConstructionScript)

(fn UpdateHoveredTile
  (bind _index (Default|GetTileIndexUnderCursor (Variables|Default|Getgrid)))
  (if (!= _index (Variables|Default|GethoveredTile))
    (Default|RemoveStatefromTile (Variables|Default|Getgrid) (Variables|Default|GethoveredTile) "NewEnumerator1")
    (Variables|Default|SethoveredTile _index)
    (Default|AddStatetoTile (Variables|Default|Getgrid) (Variables|Default|GethoveredTile) "NewEnumerator1")
    (CallFunction|OnHoveredTileChanged)))

(fn SetSelectedActions
  (params (left%20action :type BP%20Action%20Class%20Reference) (right%20action :type BP%20Action%20Class%20Reference))
  (Utilities|FlowControl|Sequence
    (:then_0
      (Utilities|IsValid (Variables|Default|GetselectedAction_leftClick)
        (:Is%20Valid
          (Actor|DestroyActor (Variables|Default|GetselectedAction_leftClick))
          (Variables|Default|SetselectedAction_leftClick 0))
        (:Is%20Not%20Valid
          _))
      (if (Utilities|IsValidClass left%20action)
        (bind _returnvalue (Game|SpawnActorfromClass left%20action (Math|Transform|MakeTransform "0, 0, 0" "0, 0, 0" "1.000000,1.000000,1.000000") "AlwaysSpawn" 0 self 0))
        (Variables|Default|SetselectedAction_leftClick _returnvalue)))
    (:then_1
      (Utilities|IsValid (Variables|Default|GetselectedAction_rightClick)
        (:Is%20Valid
          (Actor|DestroyActor (Variables|Default|GetselectedAction_rightClick))
          (Variables|Default|SetselectedAction_rightClick 0))
        (:Is%20Not%20Valid
          _))
      (if (Utilities|IsValidClass right%20action)
        (bind _returnvalue_2 (Game|SpawnActorfromClass right%20action (Math|Transform|MakeTransform "0, 0, 0" "0, 0, 0" "1.000000,1.000000,1.000000") "AlwaysSpawn" 0 self 0))
        (Variables|Default|SetselectedAction_rightClick _returnvalue_2)))
    (:then_2
      (Default|CallOnSelectedActionChanged (Variables|Default|GetselectedAction_leftClick) (Variables|Default|GetselectedAction_rightClick)))))