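; BP_Pawn is a player camera pawn that pans across the world and zooms through a spring arm.
; Forward and Right axes shift a desired location along world X and Y, while the zoom axis adjusts a clamped desired arm length.
; Tick interpolates the actor location and arm length toward those targets for smooth motion, without sweep collision.
; Pan input steps are not scaled by delta time.
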(event EventTick
  (params (DeltaSeconds :type Float%20%28single-precision%29))
  (bind _springarm (Variables|Default|GetSpringArm))
  (Variables|/Script/Engine.SpringArmComponent|SetTargetArmLength _springarm (Math|Interpolation|FInterpTo (Variables|/Script/Engine.SpringArmComponent|GetTargetArmLength _springarm) (Variables|Default|GetZoom_Desired) DeltaSeconds (Variables|Default|GetZoomInterp)))
  (Transformation|SetActorLocation (Math|Interpolation|VInterpTo (Transformation|GetActorLocation) (Variables|Default|GetLocationDesired) (Utilities|Time|GetWorldDeltaSeconds) (Variables|Default|GetLocationInterp)) false false))

(event EventBeginPlay
  (Variables|Default|SetLocationDesired (Transformation|GetActorLocation))
  (Variables|Default|SetZoom_Desired (Variables|/Script/Engine.SpringArmComponent|GetTargetArmLength (Variables|Default|GetSpringArm))))

(event Input|AxisEvents|InputAxisInputAxis_zoom
  (params (AxisValue :type Float%20%28single-precision%29))
  (Variables|Default|SetZoom_Desired (Math|Float|Clamp(Float) (+ (Variables|Default|GetZoom_Desired) (* AxisValue (Variables|Default|GetZoomSpeed))) (Variables|Default|GetZoomMin) (Variables|Default|GetZoomMax))))

(event Input|AxisEvents|InputAxisInputAxis_Forward
  (params (AxisValue :type Float%20%28single-precision%29))
  (Variables|Default|SetLocationDesired (+ (Variables|Default|GetLocationDesired) (Math|Vector|MakeVector (* AxisValue (Variables|Default|GetLocationSpeed)) 0.0 0.0))))

(event Input|AxisEvents|InputAxisInputAxis_Right
  (params (AxisValue :type Float%20%28single-precision%29))
  (Variables|Default|SetLocationDesired (+ (Variables|Default|GetLocationDesired) (Math|Vector|MakeVector 0.0 (* AxisValue (Variables|Default|GetLocationSpeed)) 0.0))))

(fn ConstructionScript)