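; Grid utility actor that draws grid cells as instances of one InstancedStaticMesh, with mesh, material, base color and collision set at init.
; A parallel InstanceIndexes array maps cell indices to instance slots for adding, replacing, removing and clearing.
; Cell states become per-instance custom data (RGB plus a filled flag) for the material, with Selected taking priority over Hovered.
; Tick is disabled on BeginPlay.
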(event EventBeginPlay
  (Actor|Tick|SetActorTickEnabled false))

(event Collision|EventActorBeginOverlap
  (params (OtherActor :type Actor%20Object%20Reference)))

(event EventTick
  (params (DeltaSeconds :type Float%20%28single-precision%29)))

(fn ConstructionScript)

(fn AddInstance
  (params (index :type Int%20Point%20Structure%20%28by%20ref%29) (InstanceTransform :type Transform%20%28by%20ref%29) (States :type Array%20of%20E_TileState%20Enums :default "NewEnumerator0"))
  (bind _instancedstaticmesh (Variables|Default|GetInstancedStaticMesh))
  (CallFunction|RemoveInstance index)
  (Components|InstancedStaticMesh|AddInstance (Variables|Default|GetInstancedStaticMesh) InstanceTransform false)
  (bind _returnvalue (Utilities|Array|Add (Variables|Default|GetinstanceIndexes) index))
  (LocalVariables|SetI _returnvalue)
  (bind (_color _isfilled) (CallFunction|GetColorfromStates States))
  (Components|InstancedStaticMesh|SetCustomDataValue _instancedstaticmesh (LocalVariables|GetI) 0 (.R (Math|Color|BreakColor _color)) false)
  (Components|InstancedStaticMesh|SetCustomDataValue _instancedstaticmesh (LocalVariables|GetI) 1 (.G (Math|Color|BreakColor _color)) false)
  (Components|InstancedStaticMesh|SetCustomDataValue _instancedstaticmesh (LocalVariables|GetI) 2 (.B (Math|Color|BreakColor _color)) false)
  (Components|InstancedStaticMesh|SetCustomDataValue _instancedstaticmesh (LocalVariables|GetI) 3 _isfilled false))

(fn RemoveInstance
  (params (index :type Int%20Point%20Structure%20%28by%20ref%29))
  (bind _instanceindexes (Variables|Default|GetinstanceIndexes))
  (if (Utilities|Array|ContainsItem _instanceindexes index)
    (Class|InstancedStaticMeshComponent|RemoveInstance (Variables|Default|GetInstancedStaticMesh) (Utilities|Array|FindItem _instanceindexes index))
    (Utilities|Array|RemoveItem (Variables|Default|GetinstanceIndexes) index)))

(fn ClearInstances
  (Components|InstancedStaticMesh|ClearInstances (Variables|Default|GetInstancedStaticMesh))
  (Utilities|Array|Clear (Variables|Default|GetinstanceIndexes)))

(fn InitGridMeshInst
  (params (mesh :type Static%20Mesh%20Object%20Reference) (material :type Material%20Interface%20Object%20Reference) (color :type Linear%20Color%20Structure) (collision :type ECollisionEnabled%20Enum :default "NoCollision"))
  (bind _instancedstaticmesh (Variables|Default|GetInstancedStaticMesh))
  (Components|StaticMesh|SetStaticMesh _instancedstaticmesh mesh)
  (Rendering|Material|SetMaterial _instancedstaticmesh 0 material)
  (Rendering|Material|SetVectorParameterValueonMaterials _instancedstaticmesh "Color" (Math|Conversions|ToVector(LinearColor) color))
  (Collision|SetCollisionEnabled _instancedstaticmesh collision))

(fn GetColorfromStates
  (params (states :type Array%20of%20E_TileState%20Enums :default "NewEnumerator0"))
  (if (== (Utilities|Array|Length states) 0)
    (return "" 0.0)
    (else
      (for _array_element (Utilities|Array|MakeArray "NewEnumerator2" "NewEnumerator1")
        (if (Utilities|Array|ContainsItem states _array_element)
          (return (Utilities|Select :Index _array_element :NewEnumerator0 "" :NewEnumerator1 "(R=0.973958,G=0.970402,B=0.142036,A=1.000000)" :NewEnumerator2 "(R=0.708333,G=0.422682,B=0.088103,A=1.000000)") 1.0)))
      (return "" 0.0))))