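; BP_gridVisual renders the grid's walkable tiles as instanced meshes.
; InitGridVisual takes the flat mesh and material from the grid's current shape data and sets up a child-actor BP_gridMeshInst with query-only collision.
; UpdateTileVisual removes a tile's instance and re-adds it with transform and states only if the tile type is walkable.
; The actor disables tick, keeps an adjustable height offset, and can clear all instances.
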(event EventBeginPlay
  (Actor|Tick|SetActorTickEnabled false))

(event Collision|EventActorBeginOverlap
  (params (OtherActor :type Actor%20Object%20Reference)))

(event EventTick
  (params (DeltaSeconds :type Float%20%28single-precision%29)))

(fn ConstructionScript)

(fn InitGridVisual
  (params (grid :type BP%20Grid%20Object%20Reference))
  (Variables|Default|SetGrid grid)
  (Variables|Default|SetgridMeshInst (.AsBP%20Grid%20Mesh%20Inst (Utilities|Casting|CastToBP_gridMeshInst (Variables|/Script/Engine.ChildActorComponent|GetChildActor (Variables|Default|GetChildActor_gridMeshInst)))))
  (Default|InitGridMeshInst :self (Variables|Default|GetgridMeshInst) :mesh (.FlatMesh (Utilities|Struct|BreakS_gridShapeData (Default|GetCurrentShapeData (Variables|Default|GetGrid)))) :material (.FlatMaterial (Utilities|Struct|BreakS_gridShapeData (Default|GetCurrentShapeData (Variables|Default|GetGrid)))) :collision "QueryOnly")
  (Transformation|SetActorLocation "0, 0, 0" false false)
  (CallFunction|SetOffsetfromGround (Variables|Default|GetoffsetFromGround)))

(fn SetOffsetfromGround
  (params (offset :type Float%20%28double-precision%29))
  (bind _returnvalue (Transformation|GetActorLocation))
  (Variables|Default|SetoffsetFromGround offset)
  (Transformation|SetActorLocation (Math|Vector|MakeVector (.x _returnvalue) (.y _returnvalue) (Variables|Default|GetoffsetFromGround)) false false))

(fn DestroyGridVisual
  (bind _gridmeshinst (Variables|Default|GetgridMeshInst))
  (Utilities|IsValid _gridmeshinst
    (:Is%20Valid
      (Default|ClearInstances _gridmeshinst))))

(fn UpdateTileVisual
  (params (data :type S%20Tile%20Data%20Structure))
  (Default|RemoveInstance (Variables|Default|GetgridMeshInst) (.index data))
  (if (CallFunction|IsTileTypeWalkable (.type data))
    (Default|AddInstance (Variables|Default|GetgridMeshInst) (.index data) (.transform data) (.states data))))