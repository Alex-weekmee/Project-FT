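; BP_GridPathfinding computes A* paths between two tiles of the Grid, with optional diagonal moves; only square grids are handled.
; Neighbors must be walkable and within one tile height of the current tile.
; Discovered tiles stay in parallel arrays sorted by estimated total cost, with straight steps winning ties, and the path is rebuilt from previous-tile links.
; Notification calls fire when search data updates or clears.
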(event EventBeginPlay)

(event Collision|EventActorBeginOverlap
  (params (OtherActor :type Actor%20Object%20Reference)))

(event EventTick
  (params (DeltaSeconds :type Float%20%28single-precision%29)))

(fn ConstructionScript)

(fn GetValidTileSibling
  (params (index :type Int%20Point%20Structure) (includeDiag :type Boolean))
  (LocalVariables|Set_inputData (.Value (Utilities|Map|Find (Variables|/Game/BP/CORE/Grid/BP_grid.BP_grid_C|GetgridTiles (Variables|Default|Getgrid)) index)))
  (bind _siblings (CallFunction|GetSiblingIndexes index includeDiag))
  (for _array_element _siblings
    (LocalVariables|Set_data (.Value (Utilities|Map|Find (Variables|/Game/BP/CORE/Grid/BP_grid.BP_grid_C|GetgridTiles (Variables|Default|Getgrid)) _array_element)))
    (if (CallFunction|IsTileTypeWalkable (.type (LocalVariables|Get_data)))
      (if (<= (Math|Float|Absolute(Float) (- (.z (.location (.transform (LocalVariables|Get_data)))) (.z (.location (.transform (LocalVariables|Get_inputData)))))) (.z (Variables|/Game/BP/CORE/Grid/BP_grid.BP_grid_C|GetTile%20Size (Variables|Default|Getgrid))))
        (Utilities|Array|Add (LocalVariables|Get_ret) (Utilities|Struct|MakeS_pathfindingData (.index (LocalVariables|Get_data)) 1 999999 999999 index)))))
  (return (LocalVariables|Get_ret)))

(fn GetSiblingIndexesSquare
  (params (index :type Int%20Point%20Structure) (includeDiag :type Boolean))
  (bind _intpoint (Utilities|Struct|MakeIntPoint 1 0))
  (bind _intpoint_2 (Utilities|Struct|MakeIntPoint 0 1))
  (bind _intpoint_3 (Utilities|Struct|MakeIntPoint -1 0))
  (bind _intpoint_4 (Utilities|Struct|MakeIntPoint 0 -1))
  (bind _returnvalue (+ index _intpoint))
  (bind _returnvalue_2 (+ index _intpoint_2))
  (bind _returnvalue_3 (+ index _intpoint_3))
  (bind _returnvalue_4 (+ index _intpoint_4))
  (bind _array (Utilities|Array|MakeArray _returnvalue _returnvalue_2 _returnvalue_3 _returnvalue_4))
  (if includeDiag
    (bind _output_get (LocalVariables|Set_ret _array))
    (Utilities|Array|AppendArray _output_get (Utilities|Array|MakeArray (+ index (Utilities|Struct|MakeIntPoint 1 1)) (+ index (Utilities|Struct|MakeIntPoint -1 1)) (+ index (Utilities|Struct|MakeIntPoint -1 -1)) (+ index (Utilities|Struct|MakeIntPoint 1 -1))))
    (return (LocalVariables|Get_ret))
    (else
      (return _array))))

(fn GetSiblingIndexes
  (params (index :type Int%20Point%20Structure) (includeDiag :type Boolean))
  (switch Utilities|FlowControl|Switch|SwitchonE_gridShape (Variables|/Game/BP/CORE/Grid/BP_grid.BP_grid_C|GetShape (Variables|Default|Getgrid))
    (:NewEnumerator1
      (return (CallFunction|GetSiblingIndexesSquare index includeDiag)))))

(fn FindPath
  (params (start :type Int%20Point%20Structure) (target :type Int%20Point%20Structure) (diagonals :type Boolean))
  (Variables|Default|SetstartIndex start)
  (Variables|Default|SettargetIndex target)
  (Variables|Default|SetincludeDiagonals diagonals)
  (CallFunction|ClearGeneratedData)
  (bind _isvalid (CallFunction|IsInputDataValid))
  (if _isvalid
    (CallFunction|DiscoverTile (Utilities|Struct|MakeS_pathfindingData (Variables|Default|GetstartIndex) 1 0 (CallFunction|GetMinCostBetween2Tiles (Variables|Default|GetstartIndex) (Variables|Default|GettargetIndex) (Variables|Default|GetincludeDiagonals)) "(X=-999,Y=-999)"))
    (while (> (Utilities|Array|Length (Variables|Default|GetdiscoveredTileIndexes)) 0)
      (bind _foundtargettile (CallFunction|AnalyseNextDiscoveredTile))
      (if _foundtargettile
        (bind _path (CallFunction|GeneratePath))
        (return _path)))
    (return (Utilities|Array|MakeArray ""))
    (else
      (return (Utilities|Array|MakeArray "")))))

(fn IsInputDataValid
  (if (!= (Variables|Default|GetstartIndex) (Variables|Default|GettargetIndex))
    (if (Default|IsTileWalkable (Variables|Default|Getgrid) (Variables|Default|GetstartIndex))
      (if (Default|IsTileWalkable (Variables|Default|Getgrid) (Variables|Default|GettargetIndex))
        (return true)
        (else
          (return false)))
      (else
        (return false)))
    (else
      (return false))))

(fn DiscoverTile
  (params (tilePathData :type S%20Pathfinding%20Data%20Structure))
  (bind _index (Utilities|Struct|BreakS_pathfindingData tilePathData))
  (Utilities|Map|Add (Variables|Default|GetpathfindingData) _index tilePathData)
  (CallFunction|InsertTileinDiscoveredArray tilePathData)
  (Default|CallOnPathfindingDataUpdated _index))

(fn GetMinCostBetween2Tiles
  (params (index1 :type Int%20Point%20Structure) (index2 :type Int%20Point%20Structure) (diagonals :type Boolean))
  (bind _returnvalue (- index1 index2))
  (bind _returnvalue_2 (- index1 index2))
  (if diagonals
    (return (Math|Integer|Max(Integer) (Math|Integer|Absolute(Integer) (.x _returnvalue_2)) (Math|Integer|Absolute(Integer) (.y _returnvalue_2))))
    (else
      (return (+ (Math|Integer|Absolute(Integer) (.x _returnvalue)) (Math|Integer|Absolute(Integer) (.y _returnvalue)))))))

(fn AnalyseNextDiscoveredTile
  (bind _tilepathdata (CallFunction|PullCheapestTileOutOfDiscoveredList))
  (bind _output_get (Variables|Default|SetcurrentDiscoveredTile _tilepathdata))
  (bind _siblings (CallFunction|GetValidTileSibling (.index (Utilities|Struct|BreakS_pathfindingData _output_get)) (Variables|Default|GetincludeDiagonals)))
  (Variables|Default|SetcurrentSiblings _siblings)
  (while (> (Utilities|Array|Length (Variables|Default|GetcurrentSiblings)) 0)
    (bind _istargettile (CallFunction|DiscoverNextSibling))
    (if _istargettile
      (return true)))
  (return false))

(fn GeneratePath
  (LocalVariables|Set_current (Variables|Default|GettargetIndex))
  (while (!= (LocalVariables|Get_current) (Variables|Default|GetstartIndex))
    (Utilities|Array|Add (LocalVariables|Get_invertedPath) (LocalVariables|Get_current))
    (LocalVariables|Set_current (.PrevIndex (Utilities|Struct|BreakS_pathfindingData (.Value (Utilities|Map|Find (Variables|Default|GetpathfindingData) (LocalVariables|Get_current)))))))
  (bind _arrayelement (Utilities|Array|ReverseforEachLoop (LocalVariables|Get_invertedPath))
    (:LoopBody
      (Utilities|Array|Add (LocalVariables|Get_ret) _arrayelement))
    (:Completed
      (return (LocalVariables|Get_ret)))))

(fn PullCheapestTileOutOfDiscoveredList
  (LocalVariables|Set_tileIndex (Utilities|Array|Get(acopy) (Variables|Default|GetdiscoveredTileIndexes)))
  (Utilities|Array|RemoveIndex (Variables|Default|GetdiscoveredTileSortingCosts))
  (Utilities|Array|RemoveIndex (Variables|Default|GetdiscoveredTileIndexes))
  (Utilities|Array|Add (Variables|Default|GetanalysedTileIndexes) (LocalVariables|Get_tileIndex))
  (return (.Value (Utilities|Map|Find (Variables|Default|GetpathfindingData) (LocalVariables|Get_tileIndex)))))

(fn DiscoverNextSibling
  (Variables|Default|SetcurrentSibling (Utilities|Array|Get(acopy) (Variables|Default|GetcurrentSiblings)))
  (Utilities|Array|RemoveIndex (Variables|Default|GetcurrentSiblings))
  (if (not (Utilities|Array|ContainsItem (Variables|Default|GetanalysedTileIndexes) (.index (Utilities|Struct|BreakS_pathfindingData (Variables|Default|GetcurrentSibling)))))
    (LocalVariables|Set_costFromStart (+ (.costFromStart (Utilities|Struct|BreakS_pathfindingData (Variables|Default|GetcurrentDiscoveredTile))) (.costToEnterTile (Utilities|Struct|BreakS_pathfindingData (Variables|Default|GetcurrentSibling)))))
    (bind _output_get (LocalVariables|Set_indexesInDiscovered (Utilities|Array|FindItem (Variables|Default|GetdiscoveredTileIndexes) (.index (Utilities|Struct|BreakS_pathfindingData (Variables|Default|GetcurrentSibling))))))
    (if (== _output_get -1)
      _
      (else
        (bind _output_get_2 (Variables|Default|SetcurrentSibling (.Value (Utilities|Map|Find (Variables|Default|GetpathfindingData) (.index (Utilities|Struct|BreakS_pathfindingData (Variables|Default|GetcurrentSibling)))))))
        (if (< (LocalVariables|Get_costFromStart) (.costFromStart (Utilities|Struct|BreakS_pathfindingData _output_get_2)))
          (Utilities|Array|RemoveIndex (Variables|Default|GetdiscoveredTileIndexes) (LocalVariables|Get_indexesInDiscovered))
          (Utilities|Array|RemoveIndex (Variables|Default|GetdiscoveredTileSortingCosts) (LocalVariables|Get_indexesInDiscovered))
          (else
            (return false)))))
    (CallFunction|DiscoverTile (Utilities|Struct|MakeS_pathfindingData (.index (Utilities|Struct|BreakS_pathfindingData (Variables|Default|GetcurrentSibling))) (.costToEnterTile (Utilities|Struct|BreakS_pathfindingData (Variables|Default|GetcurrentSibling))) (LocalVariables|Get_costFromStart) (CallFunction|GetMinCostBetween2Tiles (.index (Utilities|Struct|BreakS_pathfindingData (Variables|Default|GetcurrentSibling))) (Variables|Default|GettargetIndex) (Variables|Default|GetincludeDiagonals)) (.index (Utilities|Struct|BreakS_pathfindingData (Variables|Default|GetcurrentDiscoveredTile)))))
    (if (Class|KismetMathLibrary|EqualIntPointIntPoint (.index (Utilities|Struct|BreakS_pathfindingData (Variables|Default|GetcurrentSibling))) (Variables|Default|GettargetIndex))
      (return true)
      (else
        (return false)))
    (else
      (return false))))

(fn InsertTileinDiscoveredArray
  (params (tileData :type S%20Pathfinding%20Data%20Structure))
  (bind _discoveredtilesortingcosts (Variables|Default|GetdiscoveredTileSortingCosts))
  (LocalVariables|Set_sortingCost (CallFunction|GetTileSortingCost tileData))
  (if (== (Utilities|Array|Length (Variables|Default|GetdiscoveredTileSortingCosts)) 0)
    (Utilities|Array|Add (Variables|Default|GetdiscoveredTileSortingCosts) (LocalVariables|Get_sortingCost) :!label _label)
    (Utilities|Array|Add (Variables|Default|GetdiscoveredTileIndexes) (.index (Utilities|Struct|BreakS_pathfindingData tileData)))
    (elif (>= (LocalVariables|Get_sortingCost) (Utilities|Array|Get(acopy) _discoveredtilesortingcosts (Utilities|Array|LastIndex _discoveredtilesortingcosts)))
      (goto _label)
      (else
        (bind (_array_element _array_index) (Utilities|Array|ForEachLoopwithBreak (Variables|Default|GetdiscoveredTileSortingCosts) :!label _label_2)
          (:LoopBody
            (if (>= _array_element (LocalVariables|Get_sortingCost))
              (Utilities|Array|Insert (Variables|Default|GetdiscoveredTileSortingCosts) (LocalVariables|Get_sortingCost) _array_index)
              (Utilities|Array|Insert (Variables|Default|GetdiscoveredTileIndexes) (.index (Utilities|Struct|BreakS_pathfindingData tileData)) _array_index)
              (goto _label_2 Break))))))))

(fn ClearGeneratedData
  (Utilities|Map|Clear (Variables|Default|GetpathfindingData))
  (Utilities|Array|Clear (Variables|Default|GetdiscoveredTileSortingCosts))
  (Utilities|Array|Clear (Variables|Default|GetdiscoveredTileIndexes))
  (Utilities|Array|Clear (Variables|Default|GetanalysedTileIndexes))
  (Default|CallOnPathfindingDataCleared))

(fn IsDiagonal
  (params (index%201 :type Int%20Point%20Structure) (index%202 :type Int%20Point%20Structure))
  (bind _siblings (CallFunction|GetSiblingIndexes index%201 false))
  (return (not (Utilities|Array|ContainsItem _siblings index%202))))

(fn GetTileSortingCost
  (params (tileData :type S%20Pathfinding%20Data%20Structure%20%28by%20ref%29))
  (bind (_index _costtoentertile _costfromstart _mincosttotarget _previndex) (Utilities|Struct|BreakS_pathfindingData tileData))
  (bind (_index_2 _costtoentertile_2 _costfromstart_2 _mincosttotarget_2) (Utilities|Struct|BreakS_pathfindingData tileData))
  (return (+ (* (+ _costfromstart_2 _mincosttotarget_2) 2) (Math|Conversions|ToInteger(Boolean) (CallFunction|IsDiagonal _index _previndex)))))