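; Grid-based unit actor that builds its mesh, animation and socketed weapon from per-type unit data and walks along tile paths.
; Path following moves tile by tile on a rate-scaled timeline, adding a jump arc on height changes and firing walk and tile-reached events.
; Animation states go to the AnimBP by message, hover and selection tint materials, and a line-of-sight collision mesh matches the grid's tile shape.
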(event Custom|event_followPath
  (params (path :type Array%20of%20Int%20Point%20Structures))
  (if (> (Utilities|Array|Length path) 0)
    (Variables|Default|SetcurrentPathToFollow path)
    (Default|CallOnUnitStartedWalking self)
    (CallFunction|ContinuetoFollowPath)))

(event Custom|continueToFollowPath
  (bind _grid (Variables|Default|Getgrid))
  (bind _timeline_unitmovement (Variables|Default|GetTimeline-unitMovement))
  (bind _currentpathtofollow (Variables|Default|GetcurrentPathToFollow))
  (bind _output (Utilities|Array|Get(acopy) _currentpathtofollow))
  (bind _gridtiles (Variables|/Game/BP/CORE/Grid/BP_grid.BP_grid_C|GetgridTiles _grid))
  (bind _value (Utilities|Map|Find _gridtiles _output))
  (bind _transform (Utilities|Struct|BreakS_tileData _value))
  (if (> (Utilities|Array|Length (Variables|Default|GetcurrentPathToFollow)) 0)
    (if (!= (Utilities|Array|Get(acopy) (Variables|Default|GetcurrentPathToFollow)) (Utilities|Struct|MakeIntPoint 0 0))
      (CallFunction|SetAnimationState "NewEnumerator1")
      (Variables|Default|SetprevTransform (Transformation|GetActorTransform))
      (Variables|Default|SetnextTransform (Math|Transform|MakeTransform (.location _transform) (Math|Rotator|MakeRotator 0.0 0.0 (.yaw (Math|Rotator|FindLookatRotation (.location (Variables|Default|GetprevTransform)) (.location _transform)))) "1.000000,1.000000,1.000000"))
      (Components|Timeline|SetPlayRate _timeline_unitmovement (/ (Components|Timeline|GetTimelineLength _timeline_unitmovement) (Variables|Default|GetmoveDurationForTile)))
      (bind (_direction _locationalpha _rotationalpha _jump) (Timeline|Timeline-unitMovement PlayFromStart)
        (:Update
          (Transformation|SetActorLocationAndRotation (+ (Math|Vector|Lerp(Vector) (.location (Variables|Default|GetprevTransform)) (.location (Variables|Default|GetnextTransform)) _locationalpha) (Math|Vector|MakeVector 0.0 0.0 (select (Math|Float|NearlyEqual(Float) (.z (.location (Variables|Default|GetprevTransform))) (.z (.location (Variables|Default|GetnextTransform))) 5.0) 0.0 _jump))) (Math|Rotator|Lerp(Rotator) (.rotation (Variables|Default|GetprevTransform)) (.rotation (Variables|Default|GetnextTransform)) _rotationalpha true)))
        (:Finished
          (Default|CallOnUnitReachesNewTile self (Utilities|Array|Get(acopy) (Variables|Default|GetcurrentPathToFollow)))
          (Utilities|Array|RemoveIndex (Variables|Default|GetcurrentPathToFollow))
          (CallFunction|ContinuetoFollowPath)))
      (else
        (CallFunction|SetAnimationState "NewEnumerator0" :!label _label)
        (Default|CallOnUnitFinishedWalking self)))
    (else
      (goto _label))))

(event EventBeginPlay
  (CallFunction|SetAnimationState "NewEnumerator0"))

(fn ConstructionScript
  (bind _unitdata (CallFunction|GetDefaultUnitDatafromUnitType (Variables|Default|GetunitType)))
  (CallFunction|SetupUnitData _unitdata))

(fn ToggleWeaponVisibility
  (params (newVisibility :type Boolean) (unitType :type E_unitType%20Enum :default "NewEnumerator0"))
  (bind _childactor (Variables|Default|GetChildActor))
  (bind _childactor_2 (Variables|/Script/Engine.ChildActorComponent|GetChildActor _childactor))
  (if newVisibility
    (Class|BPIWeapon|SetWeaponVisible(Message) _childactor_2 true unitType)
    (else
      (Class|BPIWeapon|SetWeaponVisible(Message) _childactor_2 false unitType))))

(fn PullBowString
  (params (tighten :type Boolean))
  (bind _self self)
  (bind _childactor (Variables|Default|GetChildActor))
  (bind _childactor_2 (Variables|/Script/Engine.ChildActorComponent|GetChildActor _childactor))
  (if tighten
    (Class|BPIWeapon|SetStringIsTighten(Message) _childactor_2 true _self)
    (else
      (Class|BPIWeapon|SetStringIsTighten(Message) _childactor_2 false _self))))

(fn UpdateVisualifHoveredorSelected
  (Rendering|Material|SetVectorParameterValueonMaterials (Variables|Default|GetCharacter) "ColorMultiply" (Math|Conversions|ToVector(LinearColor) (* (* (select (Variables|Default|GetisHovered) 2.5 1.0) (select (Variables|Default|GetisSelected) "(R=0.000000,G=0.010536,B=0.156250,A=1.000000)" "(R=1.000000,G=1.000000,B=1.000000,A=1.000000)")) (select (Variables|Default|GetisSelected) 2.5 1.0)))))

(fn SetIsHovered
  (params (hover :type Boolean))
  (Variables|Default|SetisHovered hover)
  (CallFunction|UpdateVisualifHoveredorSelected))

(fn SetIsSelected
  (params (selected :type Boolean))
  (Variables|Default|SetisSelected selected)
  (CallFunction|UpdateVisualifHoveredorSelected))

(fn SetupUnitData
  (params (data :type S%20Unit%20Data%20Structure%20%28by%20ref%29))
  (bind _character (Variables|Default|GetCharacter))
  (bind _childactor (Variables|Default|GetChildActor))
  (bind _childactor_2 (Variables|/Script/Engine.ChildActorComponent|GetChildActor _childactor))
  (bind _asbp_weapon (Utilities|Casting|CastToBP_weapon _childactor_2))
  (bind _poseablemesh (Variables|/Game/Art/Units/BP_weapon.BP_weapon_C|GetPoseableMesh _asbp_weapon))
  (bind _output_get (Variables|Default|SetunitData data))
  (Components|SkeletalMesh|SetSkeletalMeshAsset _character (.mesh (Utilities|Struct|BreakS_unitData_assets (.assets (Utilities|Struct|BreakS_unitData _output_get)))))
  (Class|SkeletalMeshComponent|SetAnimClass _character (.animBP (Utilities|Struct|BreakS_unitData_assets (.assets (Utilities|Struct|BreakS_unitData _output_get)))))
  (LocalVariables|SetsocketTransform (Transformation|GetSocketTransform _character (.mainHand (Utilities|Struct|BreakS_unitData_assets (.assets (Utilities|Struct|BreakS_unitData _output_get)))) "RTS_World"))
  (Components|SkinnedMesh|SetSkinnedAssetandUpdate _poseablemesh (.weaponMesh (Utilities|Struct|BreakS_unitData_assets (.assets (Utilities|Struct|BreakS_unitData _output_get)))) true)
  (Transformation|SetRelativeTransform _poseablemesh (LocalVariables|GetsocketTransform) false false)
  (Transformation|AttachComponentToComponent _poseablemesh (Variables|Default|GetCharacter) (.mainHand (Utilities|Struct|BreakS_unitData_assets (.assets (Utilities|Struct|BreakS_unitData _output_get)))) "SnapToTarget" "SnapToTarget" "SnapToTarget" true)
  (Class|BPIWeapon|SetupWeaponFX(Message) _asbp_weapon)
  (CallFunction|ToggleWeaponVisibility false (Variables|Default|GetunitType))
  (CallFunction|PullBowString false))

(fn SetAnimationState
  (params (state :type E_unitAnimationState%20Enum :default "NewEnumerator0"))
  (Class|BPIUnitAnimation|SetUnitAnimationState(Message) (Components|SkeletalMesh|GetAnimInstance (Variables|Default|GetCharacter)) state))

(fn SetGrid
  (params (grid :type BP%20Grid%20Object%20Reference))
  (bind _collision_lineofsight (Variables|Default|Getcollision_LineOfSIght))
  (Variables|Default|Setgrid grid)
  (Components|StaticMesh|SetStaticMesh _collision_lineofsight (.Mesh (Utilities|Struct|BreakS_gridShapeData (Default|GetCurrentShapeData (Variables|Default|Getgrid)))))
  (Transformation|SetAbsolute _collision_lineofsight false true true)
  (Transformation|SetWorldScale3D _collision_lineofsight (Math|Vector|MakeVector (.x (/ (Variables|/Game/BP/CORE/Grid/BP_grid.BP_grid_C|GetTile%20Size (Variables|Default|Getgrid)) (.MeshSize (Utilities|Struct|BreakS_gridShapeData (Default|GetCurrentShapeData (Variables|Default|Getgrid)))))) (.y (/ (Variables|/Game/BP/CORE/Grid/BP_grid.BP_grid_C|GetTile%20Size (Variables|Default|Getgrid)) (.MeshSize (Utilities|Struct|BreakS_gridShapeData (Default|GetCurrentShapeData (Variables|Default|Getgrid)))))) (.z (Transformation|GetWorldScale (Variables|Default|Getcollision_LineOfSIght))))))