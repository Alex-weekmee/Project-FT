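; Debug actor that overlays text and highlight states on grid tiles to visualize tile and pathfinding data.
; It finds BP_grid on BeginPlay and binds to its tile, destruction and pathfinding events.
; Per walkable tile, it lazily spawns a TextRenderActor, cached by index, showing toggled index, type, cost and sort-order lines, scaled to the longest.
; Separate toggles mark discovered and analysed tiles through grid tile states.
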(event EventBeginPlay
  (bind _returnvalue (Actor|GetActorOfClass "/Game/BP/CORE/Grid/BP_grid.BP_grid_C"))
  (bind _output_get (Variables|Default|Setgrid _returnvalue))
  (EventDispatchers|BindEventtoOnTileDataUpdated _output_get (EventDispatchers|CreateEvent :!event UpdateTextonTile))
  (EventDispatchers|BindEventtoOnGridDestroyed _output_get (EventDispatchers|CreateEvent :!event ClearAllTextActors))
  (EventDispatchers|BindEventtoOnPathfindingDataUpdated (Variables|/Game/BP/CORE/Grid/BP_grid.BP_grid_C|GetgridPathfinding (Variables|Default|Getgrid)) (EventDispatchers|CreateEvent :!event UpdateStateonTile))
  (EventDispatchers|BindEventtoOnPathfindingDataCleared (Variables|/Game/BP/CORE/Grid/BP_grid.BP_grid_C|GetgridPathfinding (Variables|Default|Getgrid)) (EventDispatchers|CreateEvent :!event UpdateStateonAllTiles))
  (EventDispatchers|BindEventtoOnPathfindingDataUpdated (Variables|/Game/BP/CORE/Grid/BP_grid.BP_grid_C|GetgridPathfinding (Variables|Default|Getgrid)) (EventDispatchers|CreateEvent :!event UpdateTextonTile))
  (EventDispatchers|BindEventtoOnPathfindingDataCleared (Variables|/Game/BP/CORE/Grid/BP_grid.BP_grid_C|GetgridPathfinding (Variables|Default|Getgrid)) (EventDispatchers|CreateEvent :!event UpdateTextonAllTiles)))

(event Collision|EventActorBeginOverlap
  (params (OtherActor :type Actor%20Object%20Reference)))

(event EventTick
  (params (DeltaSeconds :type Float%20%28single-precision%29)))

(fn ConstructionScript)

(fn GetTextActor
  (params (index :type Int%20Point%20Structure))
  (bind _output_get (LocalVariables|Setactor (.Value (Utilities|Map|Find (Variables|Default|GetspawnedTexts) index))))
  (Utilities|IsValid _output_get
    (:Is%20Valid
      (return (LocalVariables|Getactor)))
    (:Is%20Not%20Valid
      (bind _returnvalue (Game|SpawnActorfromClass "/Script/Engine.TextRenderActor" (Math|Transform|MakeTransform "0, 0, 0" "0, 0, 0" "1.000000,1.000000,1.000000") "AlwaysSpawn" 0 0))
      (LocalVariables|Setactor _returnvalue)
      (Utilities|Map|Add (Variables|Default|GetspawnedTexts) index (LocalVariables|Getactor))
      (Actor|Tick|SetActorTickEnabled (LocalVariables|Getactor))
      (Collision|SetActorEnableCollision (LocalVariables|Getactor) false)
      (Rendering|Components|TextRender|SetHorizontalAlignment (Variables|/Script/Engine.TextRenderActor|GetTextRender (LocalVariables|Getactor)) "EHTA_Center")
      (Class|TextRenderComponent|SetVerticalAlignment (Variables|/Script/Engine.TextRenderActor|GetTextRender (LocalVariables|Getactor)) "EVRTA_TextCenter")
      (return (LocalVariables|Getactor)))))

(fn DestroyTextActor
  (params (index :type Int%20Point%20Structure))
  (bind _output_get (LocalVariables|Setactor (.Value (Utilities|Map|Find (Variables|Default|GetspawnedTexts) index))))
  (Utilities|IsValid _output_get
    (:Is%20Valid
      (Actor|DestroyActor _output_get)
      (Utilities|Map|Remove (Variables|Default|GetspawnedTexts) index))))

(fn ClearAllTextActors
  (bind _values (Utilities|Map|Values (Variables|Default|GetspawnedTexts)))
  (for _array_element _values
    (Actor|DestroyActor _array_element))
  (Utilities|Map|Clear (Variables|Default|GetspawnedTexts)))

(fn UpdateTextonTile
  (params (index :type Int%20Point%20Structure))
  (bind _grid (Variables|Default|Getgrid))
  (bind _gridpathfinding (Variables|/Game/BP/CORE/Grid/BP_grid.BP_grid_C|GetgridPathfinding _grid))
  (if (CallFunction|WanttoDisplayAnyText)
    (LocalVariables|Set_index index)
    (if (.ReturnValue (Utilities|Map|Find (Variables|/Game/BP/CORE/Grid/BP_grid.BP_grid_C|GetgridTiles (Variables|Default|Getgrid)) (LocalVariables|Get_index)))
      (bind _output_get (LocalVariables|Set_data (.Value (Utilities|Map|Find (Variables|/Game/BP/CORE/Grid/BP_grid.BP_grid_C|GetgridTiles (Variables|Default|Getgrid)) (LocalVariables|Get_index)))))
      (if (CallFunction|IsTileTypeWalkable (.type _output_get))
        (Utilities|FlowControl|Sequence
          (:then_0
            (Utilities|FlowControl|Sequence
              (:then_0
                (if (Variables|Default|GetShow%20Tile%20Indexes)
                  (Utilities|Array|Add (LocalVariables|Get_text) (Utilities|String|Append (Utilities|String|ToString(Integer) (.x (LocalVariables|Get_index))) ":" (Utilities|String|ToString(Integer) (.y (LocalVariables|Get_index)))))
                  (Utilities|Array|Add (LocalVariables|Get_textLengths) (Utilities|String|Len (Utilities|String|Append (Utilities|String|ToString(Integer) (.x (LocalVariables|Get_index))) ":" (Utilities|String|ToString(Integer) (.y (LocalVariables|Get_index))))))))
              (:then_1
                (if (Variables|Default|GetshowTileType)
                  (if (Utilities|Enum|NotEqual(Enum) (.type (LocalVariables|Get_data)) "NewEnumerator1")
                    (Utilities|Array|Add (LocalVariables|Get_text) (Utilities|String|EnumtoString (.type (LocalVariables|Get_data))))
                    (Utilities|Array|Add (LocalVariables|Get_textLengths) (Utilities|String|Len (Utilities|String|EnumtoString (.type (LocalVariables|Get_data))))))))
              (:then_2
                (if (Math|Boolean|ORBoolean (Variables|Default|GetshowCostToEnterTile) (Variables|Default|GetshowMinCostToTarget) (Variables|Default|GetshowCostFromStart) (Variables|Default|GetshowSortOrder))
                  (if (.ReturnValue (Utilities|Map|Find (Variables|/Game/BP/CORE/Grid/BP_GridPathfinding.BP_GridPathfinding_C|GetpathfindingData (Variables|/Game/BP/CORE/Grid/BP_grid.BP_grid_C|GetgridPathfinding (Variables|Default|Getgrid))) (LocalVariables|Get_index)))
                    (LocalVariables|Set_pathfindingData (.Value (Utilities|Map|Find (Variables|/Game/BP/CORE/Grid/BP_GridPathfinding.BP_GridPathfinding_C|GetpathfindingData (Variables|/Game/BP/CORE/Grid/BP_grid.BP_grid_C|GetgridPathfinding (Variables|Default|Getgrid))) (LocalVariables|Get_index))))
                    (Utilities|FlowControl|Sequence
                      (:then_0
                        (if (Variables|Default|GetshowCostToEnterTile)
                          (Utilities|Array|Add (LocalVariables|Get_text) (Utilities|String|Append "Enter: " (Utilities|String|ToString(Integer) (.costToEnterTile (Utilities|Struct|BreakS_pathfindingData (LocalVariables|Get_pathfindingData))))))
                          (Utilities|Array|Add (LocalVariables|Get_textLengths) (Utilities|String|Len (Utilities|String|Append "Enter: " (Utilities|String|ToString(Integer) (.costToEnterTile (Utilities|Struct|BreakS_pathfindingData (LocalVariables|Get_pathfindingData)))))))))
                      (:then_1
                        (if (Variables|Default|GetshowMinCostToTarget)
                          (if (!= (.minCostToTarget (Utilities|Struct|BreakS_pathfindingData (LocalVariables|Get_pathfindingData))) 999999)
                            (Utilities|Array|Add (LocalVariables|Get_text) (Utilities|String|Append "Min: " (Utilities|String|ToString(Integer) (.minCostToTarget (Utilities|Struct|BreakS_pathfindingData (LocalVariables|Get_pathfindingData))))))
                            (Utilities|Array|Add (LocalVariables|Get_textLengths) (Utilities|String|Len (Utilities|String|Append "Min: " (Utilities|String|ToString(Integer) (.minCostToTarget (Utilities|Struct|BreakS_pathfindingData (LocalVariables|Get_pathfindingData))))))))))
                      (:then_2
                        (if (Variables|Default|GetshowCostFromStart)
                          (if (!= (.costFromStart (Utilities|Struct|BreakS_pathfindingData (LocalVariables|Get_pathfindingData))) 999999)
                            (Utilities|Array|Add (LocalVariables|Get_text) (Utilities|String|Append "Start: " (Utilities|String|ToString(Integer) (.costFromStart (Utilities|Struct|BreakS_pathfindingData (LocalVariables|Get_pathfindingData))))))
                            (Utilities|Array|Add (LocalVariables|Get_textLengths) (Utilities|String|Len (Utilities|String|Append "Start: " (Utilities|String|ToString(Integer) (.costFromStart (Utilities|Struct|BreakS_pathfindingData (LocalVariables|Get_pathfindingData))))))))))
                      (:then_3
                        (if (Variables|Default|GetshowSortOrder)
                          (if (!= (Utilities|Array|FindItem (Variables|/Game/BP/CORE/Grid/BP_GridPathfinding.BP_GridPathfinding_C|GetdiscoveredTileIndexes _gridpathfinding) (LocalVariables|Get_index)) -1)
                            (Utilities|Array|Add (LocalVariables|Get_text) (Utilities|String|Append "Sort: " (Utilities|String|ToString(Integer) (Utilities|Array|FindItem (Variables|/Game/BP/CORE/Grid/BP_GridPathfinding.BP_GridPathfinding_C|GetdiscoveredTileIndexes _gridpathfinding) (LocalVariables|Get_index))) "( " (Utilities|String|ToString(Integer) (Utilities|Array|Get(acopy) (Variables|/Game/BP/CORE/Grid/BP_GridPathfinding.BP_GridPathfinding_C|GetdiscoveredTileSortingCosts _gridpathfinding) (Utilities|Array|FindItem (Variables|/Game/BP/CORE/Grid/BP_GridPathfinding.BP_GridPathfinding_C|GetdiscoveredTileIndexes _gridpathfinding) (LocalVariables|Get_index)))) " )"))
                            (Utilities|Array|Add (LocalVariables|Get_textLengths) (Utilities|String|Len (Utilities|String|Append "Sort: " (Utilities|String|ToString(Integer) (Utilities|Array|FindItem (Variables|/Game/BP/CORE/Grid/BP_GridPathfinding.BP_GridPathfinding_C|GetdiscoveredTileIndexes _gridpathfinding) (LocalVariables|Get_index))) "( " (Utilities|String|ToString(Integer) (Utilities|Array|Get(acopy) (Variables|/Game/BP/CORE/Grid/BP_GridPathfinding.BP_GridPathfinding_C|GetdiscoveredTileSortingCosts _gridpathfinding) (Utilities|Array|FindItem (Variables|/Game/BP/CORE/Grid/BP_GridPathfinding.BP_GridPathfinding_C|GetdiscoveredTileIndexes _gridpathfinding) (LocalVariables|Get_index)))) " )"))))))))))))
          (:then_1
            (if (> (Utilities|Array|Length (LocalVariables|Get_text)) 0)
              (bind _textrenderactor (CallFunction|GetTextActor (LocalVariables|Get_index)))
              (LocalVariables|Set_textActor _textrenderactor)
              (Rendering|Components|TextRender|SetText (Variables|/Script/Engine.TextRenderActor|GetTextRender (LocalVariables|Get_textActor)) (Utilities|Text|ToText(String) (Utilities|String|JoinStringArray (LocalVariables|Get_text) "  
")))
              (Transformation|SetActorTransform (LocalVariables|Get_textActor) (Math|Transform|MakeTransform (+ (.location (.transform (LocalVariables|Get_data))) "0.000000,0.000000,1.000000") "90.000000,180.000000,0.000000" (Math|Conversions|ToVector(Float) (/ (.y (Variables|/Game/BP/CORE/Grid/BP_grid.BP_grid_C|GetTile%20Size (Variables|Default|Getgrid))) (* (.MaxValue (Math|Integer|MaxOfIntArray (LocalVariables|Get_textLengths))) 15.0)))))
              (else
                (CallFunction|DestroyTextActor (LocalVariables|Get_index))))))
        (else
          (CallFunction|DestroyTextActor (LocalVariables|Get_index) :!label _label)))
      (else
        (goto _label)))))

(fn SetShowTileTexts
  (params (showTileIndexes :type Boolean) (showCostToEnterTile :type Boolean) (showMinCostToTarget :type Boolean) (showCostFromStart :type Boolean) (showSortOrder :type Boolean) (showTileType :type Boolean))
  (Variables|Default|SetShow%20Tile%20Indexes showTileIndexes)
  (Variables|Default|SetshowCostToEnterTile showCostToEnterTile)
  (Variables|Default|SetshowMinCostToTarget showMinCostToTarget)
  (Variables|Default|SetshowCostFromStart showCostFromStart)
  (Variables|Default|SetshowSortOrder showSortOrder)
  (Variables|Default|SetshowTileType showTileType)
  (CallFunction|UpdateTextonAllTiles))

(fn UpdateTextonAllTiles
  (if (CallFunction|WanttoDisplayAnyText)
    (bind _keys (Utilities|Map|Keys (Variables|/Game/BP/CORE/Grid/BP_grid.BP_grid_C|GetgridTiles (Variables|Default|Getgrid))))
    (for _array_element _keys
      (CallFunction|UpdateTextonTile _array_element))
    (else
      (CallFunction|ClearAllTextActors))))

(fn WanttoDisplayAnyText
  (return (Math|Boolean|ORBoolean (Variables|Default|GetShow%20Tile%20Indexes) (Variables|Default|GetshowCostToEnterTile) (Variables|Default|GetshowMinCostToTarget) (Variables|Default|GetshowCostFromStart) (Variables|Default|GetshowSortOrder) (Variables|Default|GetshowTileType))))

(fn UpdateStateonTile
  (params (index :type Int%20Point%20Structure))
  (Utilities|FlowControl|Sequence
    (:then_0
      (if (Variables|Default|GetshowDiscoveredTiles)
        (if (Utilities|Array|ContainsItem (Variables|/Game/BP/CORE/Grid/BP_GridPathfinding.BP_GridPathfinding_C|GetdiscoveredTileIndexes (Variables|/Game/BP/CORE/Grid/BP_grid.BP_grid_C|GetgridPathfinding (Variables|Default|Getgrid))) index)
          (Default|AddStatetoTile (Variables|Default|Getgrid) index "NewEnumerator5")
          (else
            (Default|RemoveStatefromTile (Variables|Default|Getgrid) index "NewEnumerator5" :!label _label)))
        (else
          (goto _label))))
    (:then_1
      (if (Variables|Default|GetshowAnalysedTiles)
        (if (Utilities|Array|ContainsItem (Variables|/Game/BP/CORE/Grid/BP_GridPathfinding.BP_GridPathfinding_C|GetanalysedTileIndexes (Variables|/Game/BP/CORE/Grid/BP_grid.BP_grid_C|GetgridPathfinding (Variables|Default|Getgrid))) index)
          (Default|AddStatetoTile (Variables|Default|Getgrid) index "NewEnumerator6")
          (else
            (Default|RemoveStatefromTile (Variables|Default|Getgrid) index "NewEnumerator6" :!label _label_2)))
        (else
          (goto _label_2))))))

(fn UpdateStateonAllTiles
  (bind _grid (Variables|Default|Getgrid))
  (if (or (Variables|Default|GetshowDiscoveredTiles) (Variables|Default|GetshowAnalysedTiles))
    (bind _keys (Utilities|Map|Keys (Variables|/Game/BP/CORE/Grid/BP_grid.BP_grid_C|GetgridTiles (Variables|Default|Getgrid))))
    (for _array_element _keys
      (CallFunction|UpdateStateonTile _array_element))
    (else
      (Default|ClearStatefromTiles _grid "NewEnumerator5")
      (Default|ClearStatefromTiles _grid "NewEnumerator6"))))

(fn SetShowTileStates
  (params (showDiscoveredTiles :type Boolean) (showAnalysedTiles :type Boolean))
  (Variables|Default|SetshowDiscoveredTiles showDiscoveredTiles)
  (Variables|Default|SetshowAnalysedTiles showAnalysedTiles)
  (CallFunction|UpdateStateonAllTiles))