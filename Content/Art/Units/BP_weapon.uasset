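; Unit weapon Blueprint with a poseable mesh and an arrow, serving as a Soldier's weapon with a trail or an Archer's bow.
; On BeginPlay it attaches a hidden trail effect between the trail sockets, sized to their distance, and shows it for a timed window when a Soldier's weapon becomes visible.
; While the string is tightened, Tick pins the String bone and arrow to the unit's right-hand socket; otherwise it resets the string and hides the arrow.
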(event EventBeginPlay
  (bind _poseablemesh (Variables|Default|GetPoseableMesh))
  (bind _returnvalue (Transformation|GetSocketLocation _poseablemesh "trail_top"))
  (bind _returnvalue_2 (Transformation|GetSocketLocation _poseablemesh "trail_bottom"))
  (bind _returnvalue_3 (- _returnvalue _returnvalue_2))
  (bind _returnvalue_4 (Niagara|SpawnSystemAttached "/Game/Art/Effects/fx_trail.fx_trail" _poseablemesh "None" (/ (+ _returnvalue _returnvalue_2) 2.0) (Math|Rotator|MakeRotfromZ _returnvalue_3) "KeepWorldPosition" false))
  (bind _output_get (Variables|Default|SetFX _returnvalue_4))
  (Rendering|SetVisibility _output_get false false)
  (Effects|Components|ParticleSystem|SetFloatParameter _output_get "TrailWidth" (Math|Vector|VectorLength _returnvalue_3)))

(event Collision|EventActorBeginOverlap
  (params (OtherActor :type Actor%20Object%20Reference)))

(event EventTick
  (params (DeltaSeconds :type Float%20%28single-precision%29))
  (bind _poseablemesh (Variables|Default|GetPoseableMesh))
  (bind _unit_ref (Variables|Default|GetUnit%20Ref))
  (bind _arrow (Variables|Default|Getarrow))
  (bind _character (Variables|/Game/BP/CORE/Units/BP_unit.BP_unit_C|GetCharacter _unit_ref))
  (bind _returnvalue (Transformation|GetSocketTransform _character "hand_rSocket" "RTS_World"))
  (if (Variables|Default|GetTighten)
    (Class|PoseableMeshComponent|SetBoneLocationbyName _poseablemesh "String" (.location _returnvalue) "WorldSpace")
    (Rendering|SetVisibility _arrow true false)
    (Transformation|SetWorldLocation _arrow (.location _returnvalue) false false)
    (else
      (Class|PoseableMeshComponent|SetBoneLocationbyName _poseablemesh "String" "0.000000,1.000000,-0.000000" "ComponentSpace")
      (Rendering|SetVisibility (Variables|Default|Getarrow) false false))))

(event EventSetStringIsTighten
  (params (tighten :type Boolean) (unitRef :type BP%20Unit%20Object%20Reference))
  (Variables|Default|SetTighten tighten)
  (Variables|Default|SetUnit%20Ref unitRef))

(event EventSetWeaponVisible
  (params (visibility :type Boolean) (unitType :type E_unitType%20Enum :default "NewEnumerator0"))
  (bind _fx (Variables|Default|GetFX))
  (bind _output_get (Variables|Default|SetVisibility visibility))
  (Rendering|SetVisibility (Variables|Default|GetPoseableMesh) _output_get false)
  (switch Utilities|FlowControl|Switch|SwitchonE_unitType unitType
    (:NewEnumerator0
      (Utilities|IsValid _fx
        (:Is%20Valid
          (if (Variables|Default|GetVisibility)
            (Utilities|FlowControl|Delay 0.7)
            (Rendering|SetVisibility _fx true false)
            (Utilities|FlowControl|Delay 0.6)
            (Rendering|SetVisibility _fx false false)
            (else
              (Rendering|SetVisibility _fx false false))))))
    (:NewEnumerator1
      (Rendering|SetVisibility (Variables|Default|Getarrow) (Variables|Default|GetVisibility) false))))

(fn ConstructionScript
  (Rendering|SetVisibility (Variables|Default|Getarrow) false false))